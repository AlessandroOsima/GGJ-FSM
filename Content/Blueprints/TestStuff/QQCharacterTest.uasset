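; QQCharacterTest is a test character that fires fireballs and is briefly stunned when one hits it.
; The ShootFireball input has its FireballLauncher launch a fireball from ShootingOrigin at a fixed velocity.
; Overlapping any Fireball disables input, then restores it after a short delay.
; Destroying the character ends the match through the game mode; two debug prints are left unconnected.
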(event `InputAction|ShootFireball`
  (params (Key :type "Key Structure" :default "AnyKey"))
  (:`Pressed`
    (`/Game/Blueprints/FireballLauncher.LaunchFireball` (`self.FireballLauncher`) (`self.ShootingOrigin`) 5000.0)))

(event `self.ReceiveActorBeginOverlap`
  (params (OtherActor :type "Actor Object Reference"))
  (cast `/Game/Blueprints/Fireball` OtherActor)
  (`self.DisableInput` null)
  (`KismetSystemLibrary.Delay` 2.0)
  (`self.EnableInput` null))

(event `self.ReceiveDestroyed`
  (`GameMode.EndMatch` (`GameplayStatics.GetGameMode` null)))

(fn `UserConstructionScript`)
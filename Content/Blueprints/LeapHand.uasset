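; Leap Motion hand actor that aims a colored ray from the palm to slow pawns or launch fireballs.
; Each tick it line-traces from the palm and moves a sphere collider to the impact point.
; Overlapping another sphere there recolors the ray and calls FindPawnInRange with a growing slowdown.
; Otherwise gripping builds charge, as does hitting the same hand, and releasing fires a fireball at fixed velocity.
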(event `self.ReceiveBeginPlay`
  (bind _ray (`self.Ray`))
  (bind _returnvalue (`PrimitiveComponent.CreateDynamicMaterialInstance` _ray 0 (`PrimitiveComponent.GetMaterial` _ray 0)))
  (set `self.Material` _returnvalue))

(event `self.ReceiveTick`
  (params (DeltaSeconds :type "Float (single-precision)"))
  (bind _returnvalue (`self.GetBoneActor` "Palm"))
  (bind _spherecollider (`self.SphereCollider`))
  (bind _spherecollider_2 (`self.SphereCollider`))
  (bind _returnvalue_2 (`self.K2_GetActorLocation` _returnvalue))
  (bind _returnvalue_3 (`self.K2_GetActorRotation` _returnvalue))
  (bind _returnvalue_4 (`SphereComponent.GetScaledSphereRadius` _spherecollider))
  (bind _rotation (.rotation (`self.GetTransform` (`self.GetBoneActor` "Palm"))))
  (bind _returnvalue_5 (`KismetMathLibrary.GetForwardVector` _returnvalue_3))
  (set `self.FluxCollision` false)
  (`SceneComponent.K2_SetWorldLocationAndRotation` (`self.Ray`) _returnvalue_2 _returnvalue_3 false true)
  (`SceneComponent.K2_AddLocalRotation` (`self.Ray`) (`KismetMathLibrary.MakeRotator` -90.0 -90.0 0.0) false false)
  (bind (_outhit _returnvalue_6) (`KismetSystemLibrary.LineTraceSingleForObjects` :`Start` (+ _returnvalue_2 (* _returnvalue_5 0.1)) :`End` (* _returnvalue_5 99999.0) :`ObjectTypes` (`|MakeArray` "ObjectTypeQuery4" "ObjectTypeQuery2" :!type "EObjectTypeQuery Enum") :`bIgnoreSelf` false))
  (if _returnvalue_6
    (bind (_bblockinghit _binitialoverlap _time _location _impactpoint _normal _impactnormal _physmat _hitactor) (`GameplayStatics.BreakHitResult` _outhit))
    ;[1 1 1] Colliding with the same hand
    (bind _asleap_motion_bone_actor (cast `LeapMotionBoneActor` _hitactor)
      (:`then`
        (if (== (`LeapMotionHandActor.HandId` (`LeapMotionBoneActor.GetHandActor` _asleap_motion_bone_actor)) (`self.HandId`))
          ;[1 1 1] Charge if collision with the same hand
          (bind _output_get (set `self.ChargeLevel` (+ (`self.ChargeLevel`) (* 1.0 DeltaSeconds)) :!label _label))
          (set `self.GrabStart` true)
          (else
            (`SceneComponent.K2_SetWorldLocation` _spherecollider_2 _impactpoint false true :!label _label_2)
            (bind (_outcomponents _returnvalue_7) (`KismetSystemLibrary.SphereOverlapComponents_NEW` _impactpoint (`SphereComponent.GetScaledSphereRadius` _spherecollider_2) (`|MakeArray` "ObjectTypeQuery7" :!type "EObjectTypeQuery Enum")))
            (if _returnvalue_7
              (for _array_element _outcomponents
                (bind _assphere_collision (cast `SphereComponent` _array_element)
                  (:`then`
                    (set `self.FluxCollision` (or (`self.FluxCollision`) (!= _assphere_collision (`self.SphereCollider`))))
                    (`KismetSystemLibrary.DrawDebugSphere` _impactpoint _returnvalue_4 12 (struct :`R` 0.47 :`G` 0.081489 :`B` 0.439881 :`A` 1.0) 0.05)
                    ;[1 1 1] Comment
                    (set `self.SlowDownLevel` (+ (`self.SlowDownLevel`) (* DeltaSeconds (`self.DecelerationAmount`))) :!label _label_3)
                    (set `self.ChargeLevel` 0.0 :!label _label_4))
                  (:`CastFailed`
                    (set `self.FluxCollision` (or (`self.FluxCollision`) false))
                    (`KismetSystemLibrary.DrawDebugSphere` _impactpoint _returnvalue_4 12 (struct :`R` 0.170342 :`G` 0.47 :`B` 0.128708 :`A` 1.0) 0.05)))))
            (if (`self.FluxCollision`)
              (`MaterialInstanceDynamic.SetVectorParameterValue` (`self.Material`) "Color" (struct :`R` 0.96 :`B` 0.946046 :`A` 1.0))
              (`self.FindPawnInRange` _impactpoint _spherecollider (`self.SlowDownLevel`) 100.0)
              (goto _label_3)
              (else
                (`MaterialInstanceDynamic.SetVectorParameterValue` (`self.Material`) "Color" (struct :`R` 0.167704 :`G` 0.88 :`B` 0.116476 :`A` 1.0))
                (set `self.SlowDownLevel` 0.0)
                (if (> (`LeapMotionFunctionLibrary.GetGrabStrength` (`self.HandId`)) 0.7)
                  (goto _label)
                  (elif (`self.GrabStart`)
                    (`/Game/Blueprints/FireballLauncher.LaunchFireball` (`self.FireballLauncher`) (`KismetMathLibrary.MakeTransform` (+ (.location (`self.GetTransform` (`self.GetBoneActor` "Palm"))) (* (`KismetMathLibrary.GetForwardVector` _rotation) 300.0)) _rotation) 1100.0)
                    (set `self.GrabStart` false)
                    (goto _label_4)
                    (else
                      (goto _label_4)))))))))
      (:`CastFailed`
        (goto _label_2)))))

(fn `UserConstructionScript`)
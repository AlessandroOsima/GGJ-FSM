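; Torch actor that lights itself after staying at or above a height threshold for a set time, and can be put out by the player.
; Tick accumulates the time, resetting it below the threshold, then calls Light.
; FSMCharacter overlap toggles input, letting the Action input or X key call TurnOff.
; OnLighted and OnTurnOff show or hide the particle system and notify the first TorchManager found in the level.
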(event `self.OnLighted`
  (`SceneComponent.SetHiddenInGame` (`self.ParticleSystem`) false true)
  (bind _outactors (`GameplayStatics.GetAllActorsOfClass` "/Game/Blueprints/TorchManager.TorchManager_C"))
  (`TorchManager.OnTorchLighted` (`KismetArrayLibrary.Array_Get` _outactors)))

(event `self.OnTurnOff`
  (`SceneComponent.SetHiddenInGame` (`self.ParticleSystem`) true true)
  (bind _outactors (`GameplayStatics.GetAllActorsOfClass` "/Game/Blueprints/TorchManager.TorchManager_C"))
  (`TorchManager.OnTorchTurnOff` (`KismetArrayLibrary.Array_Get` _outactors)))

(event `self.ReceiveBeginPlay`)

(event `self.ReceiveActorBeginOverlap`
  (params (OtherActor :type "Actor Object Reference")))

(event `self.ReceiveTick`
  (params (DeltaSeconds :type "Float (single-precision)"))
  (if (<= (`self.Height To Light`) (.z (`SceneComponent.K2_GetComponentLocation` (`self.DefaultSceneRoot`))))
    (bind _output_get (set `self.CurrentTimeToLight` (+ (`self.CurrentTimeToLight`) DeltaSeconds)))
    (if (<= (`self.TimeToLight`) _output_get)
      (`self.Light`))
    (else
      (set `self.CurrentTimeToLight` 0.0))))

(event `self.ReceiveActorBeginOverlap`
  (params (OtherActor :type "Actor Object Reference"))
  (cast `FSMCharacter` OtherActor)
  (set `self.In Radius` true)
  (`self.EnableInput` (`GameplayStatics.GetPlayerController` 0)))

(event `self.ReceiveActorEndOverlap`
  (params (OtherActor :type "Actor Object Reference"))
  (cast `FSMCharacter` OtherActor)
  (set `self.In Radius` false)
  (`self.DisableInput` (`GameplayStatics.GetPlayerController` 0)))

(event `InputAction|Action`
  (params (Key :type "Key Structure" :default "AnyKey"))
  (:`Pressed`
    (`self.TurnOff` :!label _label)))

(event `Key|X`
  (params (Key :type "Key Structure" :default "AnyKey"))
  (:`Pressed`
    (goto _label)))

(fn `UserConstructionScript`)
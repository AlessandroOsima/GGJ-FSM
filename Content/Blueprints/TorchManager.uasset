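; Torch manager that referees a timed Evil-versus-Light match and plays the soundtrack.
; Tick runs the Light countdown shown on the Timer widget, plus an Evil countdown while the torch count meets the winning threshold.
; Torch lit/off events reset the Evil countdown whenever that threshold is met.
; The first countdown to expire ends the match, shows that side's win widget and restarts the map through FSMGameMode.
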(event `self.ReceiveBeginPlay`
  ;[1 1 1] Timer widget setup
  (set `self.CurrentLightTime` (`self.TimeForLightWin`))
  (bind _returnvalue (`|CreateWidget` "/Game/Blueprints/UMG/Timer.Timer_C"))
  (bind _output_get (set `self.Timer` _returnvalue))
  (`UserWidget.AddToViewport` _returnvalue 0)
  (`UserWidget.AddToViewport` _output_get 0)
  (`AudioComponent.Play` (`self.Soundtrack`) 0.0))

(event `self.ReceiveTick`
  (params (DeltaSeconds :type "Float (single-precision)"))
  ;[1 1 1] Evil Winning Condition
  (set `/Game/Blueprints/UMG/Timer.TimeLeft` (`KismetMathLibrary.FTrunc` (`self.CurrentLightTime`)) (`self.Timer`))
  (bind _returnvalue (`self.GetTorchCount`))
  (if (<= (`self.TorchWinningNumber`) _returnvalue)
    (bind _output_get (set `self.CurrentEvilTime` (- (`self.CurrentEvilTime`) DeltaSeconds)))
    (if (<= _output_get 0.0)
      (`GameMode.EndMatch` (`GameplayStatics.GetGameMode` null))
      (if (not (`self.Game Ended`))
        (`WidgetLayoutLibrary.RemoveAllWidgets`)
        (bind _returnvalue_2 (`|CreateWidget` "/Game/Blueprints/UMG/EvilWin.EvilWin_C"))
        (`UserWidget.AddToViewport` _returnvalue_2 0)
        (set `self.Game Ended` true)
        (bind _asfsmgame_mode (cast `FSMGameMode` (`GameplayStatics.GetGameMode` null)))
        (`FSMGameMode.RestartMap` _asfsmgame_mode))
      (else
        ;[1 1 1] Light Winning Condition
        (bind _output_get_2 (set `self.CurrentLightTime` (- (`self.CurrentLightTime`) DeltaSeconds) :!label _label))
        (if (<= _output_get_2 0.0)
          (`GameMode.EndMatch` (`GameplayStatics.GetGameMode` null))
          (if (not (`self.Game Ended`))
            (`WidgetLayoutLibrary.RemoveAllWidgets`)
            (bind _returnvalue_3 (`|CreateWidget` "/Game/Blueprints/UMG/LightWin.LightWin_C"))
            (`UserWidget.AddToViewport` _returnvalue_3 0)
            (set `self.Game Ended` true)
            (bind _asfsmgame_mode_2 (cast `FSMGameMode` (`GameplayStatics.GetGameMode`)))
            (`FSMGameMode.RestartMap` _asfsmgame_mode_2)))))
    (else
      (goto _label))))

(event `self.OnTorchLightedEvent`
  ;[1 1 1] Check for winning conditions
  (bind _returnvalue (`self.GetTorchCount` :!label _label_2))
  (if (<= (`self.TorchWinningNumber`) _returnvalue)
    (set `self.CurrentEvilTime` (`self.TimeForEvilTorchWin`))))

(event `self.OnTorchTurnOffEvent`
  ;[1 1 1] Check for winning conditions
  (goto _label_2))

(fn `UserConstructionScript`)
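; Physics-driven platform Blueprint that balances itself by counteracting tilt of its Cylinder component.
; Every Tick, it reads the cylinder's world roll and pitch, zeroing either one while its magnitude is within TorqueThreshold.
; The remaining angles, scaled by StabilizationForce and DeltaSeconds, are added to the current physics angular velocity on X and Y, with no yaw contribution.
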(event `self.ReceiveTick`
  (params (DeltaSeconds :type "Float (single-precision)"))
  (bind _torque_threshold (`self.Torque Threshold`))
  (bind _roll (.roll (`SceneComponent.K2_GetComponentRotation` (`self.Cylinder`))))
  (bind _pitch (.pitch (`SceneComponent.K2_GetComponentRotation` (`self.Cylinder`))))
  ;[1 1 1] Balance the platform
  (`PrimitiveComponent.SetPhysicsAngularVelocity` (`self.Cylinder`) (* (`KismetMathLibrary.MakeVector` (`KismetMathLibrary.SelectFloat` 0.0 _roll (<= (`KismetMathLibrary.Abs` _roll) _torque_threshold)) (`KismetMathLibrary.SelectFloat` 0.0 _pitch (<= (`KismetMathLibrary.Abs` _pitch) _torque_threshold))) (* (`self.Stabilization Force`) DeltaSeconds)) true "None"))

(fn `UserConstructionScript`)